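; BP_Dynamic_Terrain is deformable terrain built from a scalar data grid and an isovalue.
; Hits from terrain-manipulating objects add a set value to grid points within a radius, destroy the object, then recalculate the mesh.
; An optional debug view, refreshed after BeginPlay and each impact, respawns one identifier actor per grid point, with its material showing whether that value exceeds the isovalue.
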(event `self.ReceiveBeginPlay`
  (`KismetSystemLibrary.DelayUntilNextTick`)
  (`self.SpawnNodeIdentifiers`))

(event `self.ReceiveActorBeginOverlap`
  (params (OtherActor :type "Actor Object Reference")))

(event `self.ReceiveHit`
  (params (MyComp :type "PrimitiveComponent Object Reference") (Other :type "Actor Object Reference") (OtherComp :type "PrimitiveComponent Object Reference") (bSelfMoved :type Boolean) (HitLocation :type "Vector Structure") (HitNormal :type "Vector Structure") (NormalImpulse :type "Vector Structure") (Hit :type "HitResult Structure (by ref)"))
  (if (`GameplayStatics.ObjectIsA` Other (`self.Terrain Manipulating Object Class`))
    (`self.AddToDataGridInRadius` (`SceneComponent.K2_GetComponentLocation` (`Actor.RootComponent` Other)) (`self.Radius Of Impact`) (`self.Value Change On Impact`))
    (`self.K2_DestroyActor` Other)
    (`self.CalculateMesh`)
    (`self.SpawnNodeIdentifiers`)))

(fn `SpawnNodeIdentifiers`
  (bind (_gridpointcount_x _gridpointcount_y _gridpointcount_z) (break `IntVector` (`self.gridPointCount`)))
  (bind _gridnodeidentifiers (`self.GridNodeIdentifiers`))
  (if (`self.SpawnGridNodeIdentifiers`)
    (for _array_element _gridnodeidentifiers
      (`self.K2_DestroyActor` _array_element))
    (`KismetArrayLibrary.Array_Clear` _gridnodeidentifiers)
    (for _index (range _gridpointcount_x)
      (for _index_2 (range _gridpointcount_y)
        (for _index_3 (range _gridpointcount_z)
          (bind _intvector (make `IntVector` _index _index_2 _index_3))
          (bind _returnvalue (`|SpawnActorFromClass` "/Game/DynamicMeshes/BP_GridNode_Identifier.BP_GridNode_Identifier_C" (`KismetMathLibrary.Conv_VectorToTransform` (`KismetMathLibrary.TransformLocation` (`SceneComponent.K2_GetComponentToWorld` (`self.RootComponent`)) (`self.GetLocalPositionOfGridPoint` _intvector))) "Undefined" "MultiplyWithRoot" null null))
          (`/Game/DynamicMeshes/BP_GridNode_Identifier.Set Active Material` _returnvalue (> (`self.GetValueOfDataGrid` _intvector) (`self.isovalue`)))
          (`KismetArrayLibrary.Array_Add` (`self.GridNodeIdentifiers`) _returnvalue))))))

(fn `UserConstructionScript`)